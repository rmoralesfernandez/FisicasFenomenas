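; BP_Constraint is a physics tether actor that links a sphere to an object with a physics constraint and a visible cable.
; On BeginPlay it attaches both to the ObjectFenomeno mesh.
; While HasEnd is false, a "Pickable" actor entering the Box is constrained and cabled instead, and the first-person character drops its held object.
; When the constraint breaks, the cable end detaches and HasEnd resets to allow another attachment.
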(event OnComponentBeginOverlap(Box)
  (params (OverlappedComponent :type Primitive%20Component%20Object%20Reference) (OtherActor :type Actor%20Object%20Reference) (OtherComp :type Primitive%20Component%20Object%20Reference) (OtherBodyIndex :type Integer) (bFromSweep :type Boolean) (SweepResult :type Hit%20Result%20Structure%20%28by%20ref%29))
  (if (not (Variables|Default|GetHasEnd))
    (if (Actor|ActorHasTag OtherActor "Pickable")
      (bind _asbp_first_person_character (Utilities|Casting|CastToBP_FirstPersonCharacter (Game|Player|GetPlayerPawn 0)))
      (Class|PhysicsConstraintComponent|SetConstrainedComponents (Variables|Default|GetPhysicsConstraint) (Variables|Default|GetSphere) "None" OtherComp "None")
      (Class|CableComponent|SetAttachEndtoComponent (Variables|Default|GetCable) OtherComp "None")
      (Default|DropObjectFenomeno _asbp_first_person_character)
      (Variables|Default|SetHasEnd true))))

(event OnConstraintBroken(PhysicsConstraint)
  (params (ConstraintIndex :type Integer))
  (Class|CableComponent|SetAttachEndtoComponent (Variables|Default|GetCable) 0 "None")
  (Variables|Default|SetHasEnd false))

(event EventBeginPlay
  (bind _objectfenomeno (Variables|Default|GetObjectFenomeno))
  (bind _staticmesh (Variables|/Game/Blueprints/Fisicas/BP_PickableObject.BP_PickableObject_C|GetStaticMesh _objectfenomeno))
  (Class|PhysicsConstraintComponent|SetConstrainedComponents (Variables|Default|GetPhysicsConstraint) (Variables|Default|GetSphere) "None" _staticmesh "None")
  (Class|CableComponent|SetAttachEndtoComponent (Variables|Default|GetCable) _staticmesh "None"))

(event Collision|EventActorBeginOverlap
  (params (OtherActor :type Actor%20Object%20Reference)))

(event EventTick
  (params (DeltaSeconds :type Float%20%28single-precision%29)))

(fn ConstructionScript)